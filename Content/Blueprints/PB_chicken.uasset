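; PB_chicken is a player-controlled chicken pawn that moves in discrete steps along the world X and Y axes.
; Releasing each of the four Move input actions adds movement input in that fixed world direction, scaled by MoveAmount, so holding a key does not repeat the step.
; Tick consumes the pending input vector and applies it directly as a swept local offset, without delta-time scaling.
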(event `self.ReceiveTick`
  (params (DeltaSeconds :type "Float (single-precision)"))
  (bind _returnvalue (`self.ConsumeMovementInputVector`))
  (`self.K2_AddActorLocalOffset` _returnvalue true))

(event `InputAction|MoveForward`
  (params (Key :type "Key Structure"))
  (:`Released`
    (`self.AddMovementInput` (1.0 0.0 0.0) (`self.Move_amount`))))

(event `InputAction|MoveBack`
  (params (Key :type "Key Structure"))
  (:`Released`
    (`self.AddMovementInput` (-1.0 0.0 0.0) (`self.Move_amount`))))

(event `InputAction|MoveRight`
  (params (Key :type "Key Structure"))
  (:`Released`
    (`self.AddMovementInput` (0.0 1.0 0.0) (`self.Move_amount`))))

(event `InputAction|MoveLeft`
  (params (Key :type "Key Structure"))
  (:`Released`
    (`self.AddMovementInput` (0.0 -1.0 0.0) (`self.Move_amount`))))

(fn `UserConstructionScript`)