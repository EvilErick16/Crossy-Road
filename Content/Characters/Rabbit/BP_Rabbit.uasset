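; Player rabbit character that hops in 100-unit steps in four directions, in the style of Crossy Road.
; Releasing a movement input turns the mesh, jumps and offsets the mesh and spring arm, with a delay flag blocking further hops.
; Tick marks it dead when mesh X exactly equals -400, then EagleKill spawns BP_Eagle and nudges the rabbit's transform once.
; The facing and rotation helper logic is unused.
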(event `self.ReceiveBeginPlay`
  (set `CharacterMovementComponent.JumpZVelocity` 200.0 (`self.CharacterMovement`)))

(event `InputAction|MoveForward`
  (params (Key :type "Key Structure"))
  ;[1 1 1] Movement
  (:`Released`
    (if (and (not (`self.is_jumping`)) (not (`self.is_dead`)))
      (set `self.is_jumping` true)
      (`SceneComponent.K2_SetRelativeRotation` :`self` (`self.Mesh`))
      (`self.Jump`)
      (`SceneComponent.K2_AddWorldOffset` (`self.Mesh`) (100.0 0.0 0.0) true false)
      (`SceneComponent.K2_AddWorldOffset` (`self.SpringArm`) (100.0 0.0 0.0) true false)
      (`KismetSystemLibrary.Delay` (`self.delay_time`))
      (set `self.is_jumping` false))))

(event `self.ReceiveTick`
  (params (DeltaSeconds :type "Float (single-precision)"))
  (bind _returnvalue_x (`KismetMathLibrary.BreakVector` (`SceneComponent.K2_GetComponentLocation` (`self.Mesh`))))
  (if (`self.is_dead`)
    _
    (elif (== _returnvalue_x -400.0)
      (set `self.is_dead` true)
      (`self.eagle_kill`))))

(event `InputAction|MoveRight`
  (params (Key :type "Key Structure"))
  ;[1 1 1] Movement
  (:`Released`
    (if (and (not (`self.is_jumping`)) (not (`self.is_dead`)))
      (set `self.is_jumping` true)
      (`SceneComponent.K2_SetRelativeRotation` (`self.Mesh`) (struct :`Yaw` 90.0) false false)
      (`self.Jump`)
      (`SceneComponent.K2_AddWorldOffset` (`self.Mesh`) (0.0 100.0 0.0) true false)
      (`SceneComponent.K2_AddWorldOffset` (`self.SpringArm`) (0.0 100.0 0.0) true false)
      (`KismetSystemLibrary.Delay` (`self.delay_time`))
      (set `self.is_jumping` false))))

(event `InputAction|MoveBack`
  (params (Key :type "Key Structure"))
  ;[1 1 1] Movement
  (:`Released`
    (if (and (not (`self.is_jumping`)) (not (`self.is_dead`)))
      (set `self.is_jumping` true)
      (`SceneComponent.K2_SetRelativeRotation` (`self.Mesh`) (struct :`Yaw` 180.0) false false)
      (`self.Jump`)
      (`SceneComponent.K2_AddWorldOffset` (`self.Mesh`) (-100.0 0.0 0.0) true false)
      (`SceneComponent.K2_AddWorldOffset` (`self.SpringArm`) (-100.0 0.0 0.0) true false)
      (`KismetSystemLibrary.Delay` (`self.delay_time`))
      (set `self.is_jumping` false))))

(event `InputAction|MoveLeft`
  (params (Key :type "Key Structure"))
  ;[1 1 1] Movement
  (:`Released`
    (if (and (not (`self.is_jumping`)) (not (`self.is_dead`)))
      (set `self.is_jumping` true)
      (`SceneComponent.K2_SetRelativeRotation` (`self.Mesh`) (struct :`Yaw` 270.0) false false)
      (`self.Jump`)
      (`SceneComponent.K2_AddWorldOffset` (`self.Mesh`) (0.0 -100.0 0.0) true false)
      (`SceneComponent.K2_AddWorldOffset` (`self.SpringArm`) (0.0 -100.0 0.0) true false)
      (`KismetSystemLibrary.Delay` (`self.delay_time`))
      (set `self.is_jumping` false))))

(fn `eagle_kill`
  (bind (_returnvalue_location _returnvalue_rotation _returnvalue_scale) (`KismetMathLibrary.BreakTransform` (`SceneComponent.K2_GetComponentToWorld` (`self.Mesh`))))
  (`|SpawnActorFromClass` "/Game/Eagle/BP_Eagle.BP_Eagle_C" (`KismetMathLibrary.MakeTransform` (`SceneComponent.K2_GetComponentLocation` (`self.eagle_spawn`)) (struct :`Yaw` 90.0) (5.0 5.0 5.0)) "Undefined" "OverrideRootScale" null null)
  (`self.K2_SetActorTransform` (`KismetMathLibrary.MakeTransform` (+ (* (`KismetMathLibrary.Normal` (`self.eagle_direction`)) (* (`GameplayStatics.GetWorldDeltaSeconds`) (`self.eagle_speed`))) _returnvalue_location) _returnvalue_rotation _returnvalue_scale)))

(fn `rotate_character`
  (params (new_rotation :type "Float (double-precision)")))

(fn `set_facing_x_direction`
  (bind (_returnvalue_x _returnvalue_y _returnvalue_z) (`KismetMathLibrary.BreakVector` (`SceneComponent.GetForwardVector` (`self.Mesh`))))
  (`|ExecutionSequence`
    (:`then_0`
      (if (== _returnvalue_z 0.0)
        (set `self.facing_x_direction` 0.0)))
    (:`then_1`
      (if (== _returnvalue_z 90.0)
        (set `self.facing_x_direction` 90.0)))
    (:`then_2`
      (if (== _returnvalue_z 180.0)
        (set `self.facing_x_direction` 180.0)))
    (:`then_3`
      (if (== _returnvalue_z 270.0)
        (set `self.facing_x_direction` 270.0)))))

(fn `UserConstructionScript`)