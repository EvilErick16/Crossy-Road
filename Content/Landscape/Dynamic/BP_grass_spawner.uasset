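; Spawner actor that builds an initial strip of 16 BP_grass tiles at BeginPlay and scatters obstacles over them.
; The first tile spawns at the origin, each next one at the previous tile's SpawnPoint, and each receives a reference to the spawner.
; Every tile gets two random bush, rock or tree side obstacles, plus weighted-random ones at its marker points.
; Each marker hit also rolls extra obstacles at fixed Y offsets on both sides.
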(event `self.ReceiveBeginPlay`
  (`self.spawn_initial_grass`))

(fn `spawn_grass`
  (params (spawn_location :type "Vector Structure"))
  (bind _returnvalue (`|SpawnActorFromClass` "/Game/Landscape/Grass/BP_grass.BP_grass_C" (`KismetMathLibrary.MakeTransform` spawn_location) "Undefined" "OverrideRootScale" null null))
  (bind _output_get (set `self.newest_grass` _returnvalue))
  (set `/Game/Landscape/Grass/BP_grass.grasss_spawner` self _output_get)
  (`self.spawn_obstacles`))

(fn `spawn_grass_at_spawn_piont`
  (`self.spawn_grass` (`SceneComponent.K2_GetComponentLocation` (`/Game/Landscape/Grass/BP_grass.spawn_point` (`self.newest_grass`)))))

(fn `spawn_initial_grass`
  (`|ExecutionSequence`
    (:`then_1`
      (for _ (range 16)
        (`/Engine/EditorBlueprintResources/StandardMacros.IsValid` (`self.newest_grass`)
          (:`Is Valid`
            (`self.spawn_grass_at_spawn_piont`))
          (:`Is Not Valid`
            (`self.spawn_grass` (0.0 0.0 0.0))))))))

(fn `spawn_obstacles`
  (bind _newest_grass (`self.newest_grass`))
  (bind (_returnvalue_x _returnvalue_y _returnvalue_z) (`KismetMathLibrary.BreakVector` (`SceneComponent.K2_GetComponentLocation` (`/Game/Landscape/Grass/BP_grass.side_obstacle_1` (`self.newest_grass`)))))
  (`|SpawnActorFromClass` (select `int` (`KismetMathLibrary.RandomIntegerInRange` 0 2) :`0` "/Game/Obstacles/Bush/BP_bush.BP_bush_C" :`1` "/Game/Obstacles/Rock/BP_rock.BP_rock_C" :`2` "/Game/Obstacles/Tree/BP_tree.BP_tree_C" :!type "Actor Class Reference") (`KismetMathLibrary.MakeTransform` (`SceneComponent.K2_GetComponentLocation` (`/Game/Landscape/Grass/BP_grass.side_obstacle_1` (`self.newest_grass`)))) "Undefined" "OverrideRootScale" null null)
  (`|SpawnActorFromClass` (select `int` (`KismetMathLibrary.RandomIntegerInRange` 0 2) :`0` "/Game/Obstacles/Bush/BP_bush.BP_bush_C" :`1` "/Game/Obstacles/Rock/BP_rock.BP_rock_C" :`2` "/Game/Obstacles/Tree/BP_tree.BP_tree_C" :!type "Actor Class Reference") (`KismetMathLibrary.MakeTransform` (`SceneComponent.K2_GetComponentLocation` (`/Game/Landscape/Grass/BP_grass.side_obstacle_2` (`self.newest_grass`)))) "Undefined" "OverrideRootScale" null null)
  (for _array_element (`|MakeArray` (`/Game/Landscape/Grass/BP_grass.obstacle_1` _newest_grass) (`/Game/Landscape/Grass/BP_grass.obstacle_2` _newest_grass) (`/Game/Landscape/Grass/BP_grass.obstacle_3` _newest_grass) (`/Game/Landscape/Grass/BP_grass.obstacle_4` _newest_grass) (`/Game/Landscape/Grass/BP_grass.obstacle_5` _newest_grass) (`/Game/Landscape/Grass/BP_grass.obstacle_6` _newest_grass) (`/Game/Landscape/Grass/BP_grass.obstacle_7` _newest_grass) (`/Game/Landscape/Grass/BP_grass.obstacle_8` _newest_grass) (`/Game/Landscape/Grass/BP_grass.obstacle_9` _newest_grass) (`/Game/Landscape/Grass/BP_grass.obstacle_10` _newest_grass) (`/Game/Landscape/Grass/BP_grass.obstacle_11` _newest_grass) (`/Game/Landscape/Grass/BP_grass.obstacle_12` _newest_grass) (`/Game/Landscape/Grass/BP_grass.obstacle_13` _newest_grass) (`/Game/Landscape/Grass/BP_grass.obstacle_14` _newest_grass))
    (if (`KismetMathLibrary.RandomBoolWithWeight` 0.2)
      (`|SpawnActorFromClass` (select `int` (`KismetMathLibrary.RandomIntegerInRange` 0 2) :`0` "/Game/Obstacles/Bush/BP_bush.BP_bush_C" :`1` "/Game/Obstacles/Rock/BP_rock.BP_rock_C" :`2` "/Game/Obstacles/Tree/BP_tree.BP_tree_C" :!type "Actor Class Reference") (`KismetMathLibrary.MakeTransform` (`SceneComponent.K2_GetComponentLocation` _array_element)) "Undefined" "OverrideRootScale" null null)
      (for _array_element_2 (`|MakeArray` 830.0 930.0 1030.0 1130.0 1230.0 1330.0 1430.0 1530.0 1630.0 1730.0 -850.0 -950.0 -1050.0 -1150.0 -1250.0 -1350.0 -1450.0 -1550.0 -1650.0 -1750.0 :!type "Float (single-precision)")
        (if (`KismetMathLibrary.RandomBoolWithWeight` 0.2)
          (`|SpawnActorFromClass` (select `int` (`KismetMathLibrary.RandomIntegerInRange` 0 2) :`0` "/Game/Obstacles/Bush/BP_bush.BP_bush_C" :`1` "/Game/Obstacles/Rock/BP_rock.BP_rock_C" :`2` "/Game/Obstacles/Tree/BP_tree.BP_tree_C" :!type "Actor Class Reference") (`KismetMathLibrary.MakeTransform` (`KismetMathLibrary.MakeVector` _returnvalue_x _array_element_2 _returnvalue_z)) "Undefined" "OverrideRootScale" null null))))))

(fn `UserConstructionScript`)